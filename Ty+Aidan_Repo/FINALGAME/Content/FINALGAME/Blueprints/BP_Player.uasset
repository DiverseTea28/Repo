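; BP_Player is the player character for a side-scrolling platformer, adding the IMC_Platforming Enhanced Input context on BeginPlay.
; Movement runs along the world X axis, snapping control rotation yaw to face the direction of travel.
; Jump uses the built-in character jump, while drop-down and interact inputs only set pressed-state flags, with no logic here consuming them.
; A quit action exits the game.
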(event `self.ReceiveBeginPlay`
  (bind _asplayer_controller (cast `PlayerController` (`self.GetController`)))
  (`EnhancedInputSubsystemInterface.AddMappingContext` (pcsubsystem `EnhancedInputLocalPlayerSubsystem` _asplayer_controller) "/Game/FINALGAME/Input/IMC_Platforming.IMC_Platforming" 0 (struct)))

(event `EnhancedInput|/Game/FINALGAME/Input/Actions/IA_Move`
  (params (ActionValue :type "Float (double-precision)") (ElapsedSeconds :type "Float (double-precision)") (TriggeredSeconds :type "Float (double-precision)") (InputAction :type "InputAction Object Reference" :default "/Game/FINALGAME/Input/Actions/IA_Move.IA_Move"))
  (:`Triggered`
    (`self.AddMovementInput` (1.0 0.0 0.0) ActionValue)
    (`Controller.SetControlRotation` (`self.GetController`) (select `bool` (> ActionValue 0.0) :`false` (`KismetMathLibrary.MakeRotator` 0.0 0.0 180.0) :`true` (`KismetMathLibrary.MakeRotator` 0.0)))))

(event `EnhancedInput|/Game/FINALGAME/Input/Actions/IA_Jump`
  (params (ActionValue :type Boolean) (ElapsedSeconds :type "Float (double-precision)") (TriggeredSeconds :type "Float (double-precision)") (InputAction :type "InputAction Object Reference" :default "/Game/FINALGAME/Input/Actions/IA_Jump.IA_Jump"))
  (:`Triggered`
    (`self.Jump`))
  (:`Completed`
    (`self.StopJumping`)))

(event `EnhancedInput|/Game/FINALGAME/Input/Actions/IA_DropDown`
  (params (ActionValue :type Boolean) (ElapsedSeconds :type "Float (double-precision)") (TriggeredSeconds :type "Float (double-precision)") (InputAction :type "InputAction Object Reference" :default "/Game/FINALGAME/Input/Actions/IA_DropDown.IA_DropDown"))
  (:`Triggered`
    (set `self.IA_DropDownPressed` true))
  (:`Completed`
    (set `self.IA_DropDownPressed` false)))

(event `EnhancedInput|/Game/FINALGAME/Input/Actions/IA_Interact`
  (params (ActionValue :type Boolean) (ElapsedSeconds :type "Float (double-precision)") (TriggeredSeconds :type "Float (double-precision)") (InputAction :type "InputAction Object Reference" :default "/Game/FINALGAME/Input/Actions/IA_Interact.IA_Interact"))
  (:`Triggered`
    (set `self.IA_InteractPressed` true))
  (:`Completed`
    (set `self.IA_InteractPressed` false)))

(event `EnhancedInput|/Game/FINALGAME/Input/Actions/IA_Quit`
  (params (ActionValue :type Boolean) (ElapsedSeconds :type "Float (double-precision)") (TriggeredSeconds :type "Float (double-precision)") (InputAction :type "InputAction Object Reference" :default "/Game/FINALGAME/Input/Actions/IA_Quit.IA_Quit"))
  (:`Triggered`
    (`KismetSystemLibrary.QuitGame` null "Quit")))

(fn `UserConstructionScript`)